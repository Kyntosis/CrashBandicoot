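; TNT crate actor that arms itself when hit with a straight downward normal, then explodes after a short countdown.
; Arming happens once, starting a timer and passing its handle through an IsArmed call.
; The timer only destroys the actor; the Destroyed event spawns BP_Explosion, so other causes of destruction also explode it.
; BeginPlay accesses the crate's timer widget and sets its Crate reference to None.
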(event `self.ReceiveBeginPlay`
  (`parent.ReceiveBeginPlay`)
  (bind _astimer_widget (cast `/Game/Crates/TimerWidget` (`WidgetComponent.GetUserWidgetObject` (`self.Widget`))))
  (set `/Game/Crates/TimerWidget.Crate` null _astimer_widget))

(event `self.ReceiveHit`
  (params (MyComp :type "PrimitiveComponent Object Reference") (Other :type "Actor Object Reference") (OtherComp :type "PrimitiveComponent Object Reference") (bSelfMoved :type Boolean) (HitLocation :type "Vector Structure") (HitNormal :type "Vector Structure") (NormalImpulse :type "Vector Structure") (Hit :type "HitResult Structure (by ref)"))
  (if (`self.Armed`)
    _
    (elif (== (.z HitNormal) -1.0)
      (set `self.Armed` true)
      (bind _returnvalue (`KismetSystemLibrary.K2_SetTimerDelegate` (delegate `Explode`) 3.0))
      (`self. IsArmed` _returnvalue))))

(event `Explode`
  (`self.K2_DestroyActor`))

(event `self.ReceiveDestroyed`
  (`|SpawnActorFromClass` "/Game/BP_Explosion.BP_Explosion_C" (`self.GetTransform`) "Undefined" "MultiplyWithRoot" null null))

(fn `UserConstructionScript`
  (`parent.UserConstructionScript`))