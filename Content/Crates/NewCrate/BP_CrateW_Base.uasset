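; BP_CrateW_Base is a breakable crate that bounces the player and drops a BP_Wumpa when broken.
; Top and bottom box overlaps launch the player character with separate velocities and decrement Hits, applying damage to itself once Hits runs out.
; Any damage spawns the Wumpa, marks the crate inactive and calls Respawn, which only hides the actor, disables its collision and unhides the decal component.
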(event `Respawn`
  (`self.SetActorHiddenInGame` self true)
  (`self.SetActorEnableCollision` self false)
  (`SceneComponent.SetHiddenInGame` (`self.Decal`) false false))

(event `self.ReceiveAnyDamage`
  (params (Damage :type "Float (single-precision)") (DamageType :type "DamageType Object Reference") (InstigatedBy :type "Controller Object Reference") (DamageCauser :type "Actor Object Reference"))
  (`|SpawnActorFromClass` "/Game/Blueprints/BP_Wumpa.BP_Wumpa_C" (`self.GetTransform`) "Undefined" "MultiplyWithRoot" null null)
  (set `self.IsActive` false)
  (`self.Respawn`))

(event `self.BoxCollisionUp.OnComponentBeginOverlap`
  (params (OverlappedComponent :type "PrimitiveComponent Object Reference") (OtherActor :type "Actor Object Reference") (OtherComp :type "PrimitiveComponent Object Reference") (OtherBodyIndex :type Integer) (bFromSweep :type Boolean) (SweepResult :type "HitResult Structure (by ref)"))
  (bind _asbp_third_person_character (cast `/Game/ThirdPerson/Blueprints/BP_ThirdPersonCharacter` (`GameplayStatics.GetPlayerCharacter` 0)))
  (if (== _asbp_third_person_character OtherActor)
    (`Character.LaunchCharacter` _asbp_third_person_character (`self.Launch Velocity Up`) false false)
    (bind _result (`/Engine/EditorBlueprintResources/StandardMacros.DecrementInt` (`self.Hits`))
      (:`  `
        (if (<= _result 0)
          (`GameplayStatics.ApplyDamage` self 1.0))))))

(event `self.BoxCollisionDown.OnComponentBeginOverlap`
  (params (OverlappedComponent :type "PrimitiveComponent Object Reference") (OtherActor :type "Actor Object Reference") (OtherComp :type "PrimitiveComponent Object Reference") (OtherBodyIndex :type Integer) (bFromSweep :type Boolean) (SweepResult :type "HitResult Structure (by ref)"))
  (bind _asbp_third_person_character (cast `/Game/ThirdPerson/Blueprints/BP_ThirdPersonCharacter` (`GameplayStatics.GetPlayerCharacter` 0)))
  (if (== _asbp_third_person_character OtherActor)
    (`Character.LaunchCharacter` _asbp_third_person_character (`self.Launch Velocity Down`) false false)
    (bind _result (`/Engine/EditorBlueprintResources/StandardMacros.DecrementInt` (`self.Hits`))
      (:`  `
        (if (<= _result 0)
          (`GameplayStatics.ApplyDamage` self 1.0))))))

(fn `UserConstructionScript`)