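; BP_CrateW1_Base is a base crate that behaves as TNT or Nitro, each marked by its own widget.
; Top and bottom boxes launch the player while hits remain; the first hit arms TNT, starting an Explode timer passed to CallIsArmed.
; Nitro explodes on top contact, while crates with neither flag become TNT when touched.
; Damage also triggers Explode, which spawns BP_Explosion; Respawn hides the crate and disables collision.
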(event `self.ReceiveBeginPlay`
  (set `self.Armed` false)
  (if (`self.IsTNT`)
    (set `self.TNTTimer` (`self.StartingTimer`))
    (`SceneComponent.SetVisibility` (`self.WidgetTNT`) true false)
    (`SceneComponent.SetVisibility` (`self.WidgetNitro`) false false)
    (else
      (`SceneComponent.SetVisibility` (`self.WidgetTNT`) false false)
      (`SceneComponent.SetVisibility` (`self.WidgetNitro`) true false))))

(event `Respawn`
  (`self.SetActorHiddenInGame` self true)
  (`self.SetActorEnableCollision` self false))

(event `self.BoxCollisionUp.OnComponentBeginOverlap`
  (params (OverlappedComponent :type "PrimitiveComponent Object Reference") (OtherActor :type "Actor Object Reference") (OtherComp :type "PrimitiveComponent Object Reference") (OtherBodyIndex :type Integer) (bFromSweep :type Boolean) (SweepResult :type "HitResult Structure (by ref)"))
  (bind _asbp_third_person_character (cast `/Game/ThirdPerson/Blueprints/BP_ThirdPersonCharacter` (`GameplayStatics.GetPlayerCharacter` 0)))
  (if (== _asbp_third_person_character OtherActor)
    (if (`self.IsTNT`)
      (if (>= (`self.Hits`) 1) :!label _label
        (`Character.LaunchCharacter` _asbp_third_person_character (`self.Launch Velocity Up`) false false)
        (`/Engine/EditorBlueprintResources/StandardMacros.DecrementInt` (`self.Hits`) :!label _label_2
          (:`  `
            (if (not (`self.Armed`))
              (set `self.Armed` true)
              (bind _returnvalue (`KismetSystemLibrary.K2_SetTimerDelegate` (delegate `Explode`) (`self.TNTTimer`)))
              (`self.IsArmed` _returnvalue)))))
      (elif (`self.IsNitro`)
        (`self.Explode`)
        (else
          (set `self.IsTNT` true)
          (goto _label))))))

(event `Explode`
  (`|SpawnActorFromClass` "/Game/BP_Explosion.BP_Explosion_C" (`self.GetTransform`) "Undefined" "MultiplyWithRoot" null null))

(event `self.BoxCollisionDown.OnComponentBeginOverlap`
  (params (OverlappedComponent :type "PrimitiveComponent Object Reference") (OtherActor :type "Actor Object Reference") (OtherComp :type "PrimitiveComponent Object Reference") (OtherBodyIndex :type Integer) (bFromSweep :type Boolean) (SweepResult :type "HitResult Structure (by ref)"))
  (bind _asbp_third_person_character (cast `/Game/ThirdPerson/Blueprints/BP_ThirdPersonCharacter` (`GameplayStatics.GetPlayerCharacter` 0)))
  (if (== _asbp_third_person_character OtherActor)
    (if (`self.IsTNT`)
      (if (>= (`self.Hits`) 1) :!label _label_3
        (`Character.LaunchCharacter` _asbp_third_person_character (`self.Launch Velocity Down`) false false)
        (goto _label_2))
      (elif (not (`self.IsNitro`))
        (set `self.IsTNT` true)
        (goto _label_3)))))

(event `self.ReceiveAnyDamage`
  (params (Damage :type "Float (single-precision)") (DamageType :type "DamageType Object Reference") (InstigatedBy :type "Controller Object Reference") (DamageCauser :type "Actor Object Reference"))
  (`self.Explode`))

(fn `UserConstructionScript`)