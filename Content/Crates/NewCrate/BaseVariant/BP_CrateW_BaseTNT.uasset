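; Base TNT crate that bounces the player on contact and spawns BP_Explosion when set off.
; Top and bottom boxes launch the player and decrement Hits; at zero, top contact starts a fuse timer, bottom contact explodes immediately.
; The fuse handle goes out through CallIsArmed, and the timer widget receives a crate reference on BeginPlay.
; Any damage also explodes it, first calling Respawn, which disarms it, disables collision and hides cube and widget.
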(event `self.ReceiveBeginPlay`
  (bind _astimer_widget_tnt2 (cast `/Game/Crates/TimerWidgetTNT2` (`WidgetComponent.GetUserWidgetObject` (`self.TNTWidget`))))
  (set `/Game/Crates/TimerWidgetTNT2.Crate` self _astimer_widget_tnt2))

(event `Respawn`
  (`self.SetActorHiddenInGame` self false)
  (`self.SetActorEnableCollision` self false)
  (`SceneComponent.SetHiddenInGame` (`self.Cube`) true false)
  (set `self.Armed` false)
  (`SceneComponent.SetHiddenInGame` (`self.TNTWidget`) true false))

(event `self.ReceiveAnyDamage`
  (params (Damage :type "Float (single-precision)") (DamageType :type "DamageType Object Reference") (InstigatedBy :type "Controller Object Reference") (DamageCauser :type "Actor Object Reference"))
  (set `self.IsActive` false)
  (`self.Respawn`)
  (`self.Explode`))

(event `self.BoxCollisionUp.OnComponentBeginOverlap`
  (params (OverlappedComponent :type "PrimitiveComponent Object Reference") (OtherActor :type "Actor Object Reference") (OtherComp :type "PrimitiveComponent Object Reference") (OtherBodyIndex :type Integer) (bFromSweep :type Boolean) (SweepResult :type "HitResult Structure (by ref)"))
  (bind _asbp_third_person_character (cast `/Game/ThirdPerson/Blueprints/BP_ThirdPersonCharacter` (`GameplayStatics.GetPlayerCharacter` 0)))
  (if (== _asbp_third_person_character OtherActor)
    (if (>= (`self.Hits`) 1)
      (`Character.LaunchCharacter` _asbp_third_person_character (`self.Launch Velocity Up`) false false)
      (bind _result (`/Engine/EditorBlueprintResources/StandardMacros.DecrementInt` (`self.Hits`))
        (:`  `
          (if (<= _result 0)
            (if (not (`self.Armed`))
              (set `self.Armed` true)
              (bind _returnvalue (`KismetSystemLibrary.K2_SetTimerDelegate` (delegate `Explode`) (`self.TntTimer`)))
              (`self.IsArmed` _returnvalue))))))))

(event `Explode`
  (`|SpawnActorFromClass` "/Game/BP_Explosion.BP_Explosion_C" (`self.GetTransform`) "Undefined" "MultiplyWithRoot" null null))

(event `self.BoxCollisionDown.OnComponentBeginOverlap`
  (params (OverlappedComponent :type "PrimitiveComponent Object Reference") (OtherActor :type "Actor Object Reference") (OtherComp :type "PrimitiveComponent Object Reference") (OtherBodyIndex :type Integer) (bFromSweep :type Boolean) (SweepResult :type "HitResult Structure (by ref)"))
  (bind _asbp_third_person_character (cast `/Game/ThirdPerson/Blueprints/BP_ThirdPersonCharacter` (`GameplayStatics.GetPlayerCharacter` 0)))
  (if (== _asbp_third_person_character OtherActor)
    (if (>= (`self.Hits`) 1)
      (`Character.LaunchCharacter` _asbp_third_person_character (`self.Launch Velocity Down`) false false)
      (bind _result (`/Engine/EditorBlueprintResources/StandardMacros.DecrementInt` (`self.Hits`))
        (:`  `
          (if (<= _result 0)
            (if (not (`self.Armed`))
              (set `self.Armed` true)
              (`self.Explode`))))))))

(fn `UserConstructionScript`)