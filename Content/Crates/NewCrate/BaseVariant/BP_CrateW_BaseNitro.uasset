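; Nitro crate Blueprint that goes off when it takes any damage or the player character hits its cube.
; Both triggers call Respawn, which despite its name disables collision, clears Armed and hides the cube and nitro widget, then call Explode.
; Explode spawns an actor at the crate's transform; the crate itself is never destroyed.
; Only the damage path also clears IsActive, which is set on BeginPlay.
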(event `self.ReceiveBeginPlay`
  (set `self.IsActive` true))

(event `Respawn`
  (`self.SetActorHiddenInGame` self false)
  (`self.SetActorEnableCollision` self false)
  (`SceneComponent.SetHiddenInGame` (`self.Cube`) true false)
  (set `self.Armed` false)
  (`SceneComponent.SetHiddenInGame` (`self.NitroWidget`) true false))

(event `self.ReceiveAnyDamage`
  (params (Damage :type "Float (single-precision)") (DamageType :type "DamageType Object Reference") (InstigatedBy :type "Controller Object Reference") (DamageCauser :type "Actor Object Reference"))
  (set `self.IsActive` false)
  (`self.Respawn`)
  (`self.Explode`))

(event `Explode`
  (`|SpawnActorFromClass` "/Game/BP_Explosion.BP_Explosion_C" (`self.GetTransform`) "Undefined" "MultiplyWithRoot" null null))

(event `self.Cube.OnComponentHit`
  (params (HitComponent :type "PrimitiveComponent Object Reference") (OtherActor :type "Actor Object Reference") (OtherComp :type "PrimitiveComponent Object Reference") (NormalImpulse :type "Vector Structure") (Hit :type "HitResult Structure (by ref)"))
  (bind _asbp_third_person_character (cast `/Game/ThirdPerson/Blueprints/BP_ThirdPersonCharacter` (`GameplayStatics.GetPlayerCharacter` 0)))
  (if (== _asbp_third_person_character OtherActor)
    (`self.Respawn`)
    (`self.Explode`)))

(fn `UserConstructionScript`)