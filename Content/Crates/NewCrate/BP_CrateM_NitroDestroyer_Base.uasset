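; Base nitro destroyer crate that, once activated by the player, sets off every nitro crate in the level.
; BeginPlay caches all BP_CrateW_BaseNitro actors; the first player damage calls Respawn on each and spawns explosions at their transforms.
; Top and bottom overlap boxes launch the player (top skipped for launchers) and count down Hits, self-applying damage at zero.
; Its own Respawn hides it, disables collision and unhides a decal; SpawnCrates is empty.
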(event `DespawnCrates`
  ;[1 1 1] Despawn Crates
  (`|ExecutionSequence`
    (:`then_0`
      (for _array_element (`self.ArrayNitro`)
        (`/Game/Crates/NewCrate/BaseVariant/BP_CrateW_BaseNitro.Respawn` _array_element)
        (`|SpawnActorFromClass` "/Game/BP_Explosion.BP_Explosion_C" (`self.GetTransform` _array_element) "Undefined" "MultiplyWithRoot" null null)))))

(event `SpawnCrates`
  ;[1 1 1] SpawnCrates
  (`|ExecutionSequence`))

(event `self.ReceiveBeginPlay`
  (bind _outactors (`GameplayStatics.GetAllActorsOfClass` "/Game/Crates/NewCrate/BaseVariant/BP_CrateW_BaseNitro.BP_CrateW_BaseNitro_C"))
  (set `self.ArrayNitro` _outactors))

(event `Respawn`
  (`self.SetActorHiddenInGame` self true)
  (`self.SetActorEnableCollision` self false)
  (`SceneComponent.SetHiddenInGame` (`self.Decal`) false false))

(event `self.ReceiveAnyDamage`
  (params (Damage :type "Float (single-precision)") (DamageType :type "DamageType Object Reference") (InstigatedBy :type "Controller Object Reference") (DamageCauser :type "Actor Object Reference"))
  (if (== DamageCauser (`GameplayStatics.GetPlayerCharacter` 0))
    (`/Engine/EditorBlueprintResources/StandardMacros.DoOnce` false
      (:`Completed`
        (set `self.CrateActivated` true)
        (`self.DespawnCrates`)))))

(event `self.BoxCollisionUp.OnComponentBeginOverlap`
  (params (OverlappedComponent :type "PrimitiveComponent Object Reference") (OtherActor :type "Actor Object Reference") (OtherComp :type "PrimitiveComponent Object Reference") (OtherBodyIndex :type Integer) (bFromSweep :type Boolean) (SweepResult :type "HitResult Structure (by ref)"))
  (bind _asbp_third_person_character (cast `/Game/ThirdPerson/Blueprints/BP_ThirdPersonCharacter` (`GameplayStatics.GetPlayerCharacter` 0)))
  (if (== _asbp_third_person_character OtherActor)
    (if (not (`self.IsLauncher`))
      (`Character.LaunchCharacter` _asbp_third_person_character (`self.Launch Velocity Up`) false false)
      (bind _result (`/Engine/EditorBlueprintResources/StandardMacros.DecrementInt` (`self.Hits`))
        (:`  `
          (if (<= _result 0)
            (`GameplayStatics.ApplyDamage` self 1.0 null _asbp_third_person_character)))))))

(event `self.BoxCollisionDown.OnComponentBeginOverlap`
  (params (OverlappedComponent :type "PrimitiveComponent Object Reference") (OtherActor :type "Actor Object Reference") (OtherComp :type "PrimitiveComponent Object Reference") (OtherBodyIndex :type Integer) (bFromSweep :type Boolean) (SweepResult :type "HitResult Structure (by ref)"))
  (bind _asbp_third_person_character (cast `/Game/ThirdPerson/Blueprints/BP_ThirdPersonCharacter` (`GameplayStatics.GetPlayerCharacter` 0)))
  (if (== _asbp_third_person_character OtherActor)
    (`Character.LaunchCharacter` _asbp_third_person_character (`self.Launch Velocity Down`) false false)
    (bind _result (`/Engine/EditorBlueprintResources/StandardMacros.DecrementInt` (`self.Hits`))
      (:`  `
        (if (<= _result 0)
          (`GameplayStatics.ApplyDamage` self 1.0 null OtherActor))))))

(fn `UserConstructionScript`)