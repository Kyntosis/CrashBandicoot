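; Switch crate that turns linked wood, TNT and Nitro crates from transparent, non-colliding ghosts into solid crates.
; BeginPlay ghosts all three arrays by swapping materials and disabling collision.
; Top and bottom trigger boxes launch the player and count down Hits before applying self-damage, which fires SpawnCrates once.
; The Nitro loop in SpawnCrates is disconnected, so that array is not iterated on spawn.
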(event OnComponentBeginOverlap(BoxCollisionUp)
  (params (OverlappedComponent :type Primitive%20Component%20Object%20Reference) (OtherActor :type Actor%20Object%20Reference) (OtherComp :type Primitive%20Component%20Object%20Reference) (OtherBodyIndex :type Integer) (bFromSweep :type Boolean) (SweepResult :type Hit%20Result%20Structure%20%28by%20ref%29))
  (bind _asbp_third_person_character (Utilities|Casting|CastToBP_ThirdPersonCharacter (Game|GetPlayerCharacter 0)))
  (if (== _asbp_third_person_character OtherActor)
    (if (not (Variables|Default|GetIsLauncher))
      (Character|LaunchCharacter _asbp_third_person_character (Variables|Default|GetLaunch%20Velocity%20Up) false false)
      (bind _result (Math|Integer|DecrementInt (Variables|Default|GetHits))
        (:%20%20
          (if (<= _result 0)
            (Game|Damage|ApplyDamage self 1.0 0 _asbp_third_person_character)))))))

(event OnComponentBeginOverlap(BoxCollisionDown)
  (params (OverlappedComponent :type Primitive%20Component%20Object%20Reference) (OtherActor :type Actor%20Object%20Reference) (OtherComp :type Primitive%20Component%20Object%20Reference) (OtherBodyIndex :type Integer) (bFromSweep :type Boolean) (SweepResult :type Hit%20Result%20Structure%20%28by%20ref%29))
  (bind _asbp_third_person_character (Utilities|Casting|CastToBP_ThirdPersonCharacter (Game|GetPlayerCharacter 0)))
  (if (== _asbp_third_person_character OtherActor)
    (Character|LaunchCharacter _asbp_third_person_character (Variables|Default|GetLaunch%20Velocity%20Down) false false)
    (bind _result (Math|Integer|DecrementInt (Variables|Default|GetHits))
      (:%20%20
        (if (<= _result 0)
          (Game|Damage|ApplyDamage self 1.0 0 OtherActor))))))

(event Custom|Respawn
  (bind _self self)
  (Rendering|SetActorHiddenInGame _self true)
  (Collision|SetActorEnableCollision _self false)
  (Development|SetHiddeninGame (Variables|Default|GetDecal) false false))

(event Custom|DespawnCrates
  ;[1 1 1] Despawn Crates
  (Utilities|FlowControl|Sequence
    (:then_0
      (for _array_element (Variables|Default|GetArrayCrate)
        (Rendering|Material|SetMaterial (Variables|/Game/Crates/NewCrate/BP_CrateW_Base.BP_CrateW_Base_C|GetCube _array_element) 0 "/Game/Materials/M_WoodTransparent.M_WoodTransparent")
        (Collision|SetActorEnableCollision _array_element false)))
    (:then_1
      (for _array_element_2 (Variables|Default|GetArrayTNT)
        (Rendering|Material|SetMaterial (Variables|/Game/Crates/NewCrate/BaseVariant/BP_CrateW_BaseTNT.BP_CrateW_BaseTNT_C|GetCube _array_element_2) 0 "/Game/Materials/M_TNTTransparent.M_TNTTransparent")
        (Collision|SetActorEnableCollision _array_element_2 false)))
    (:then_2
      (for _array_element_3 (Variables|Default|GetArrayNitro)
        (Rendering|Material|SetMaterial (Variables|/Game/Crates/NewCrate/BaseVariant/BP_CrateW_BaseNitro.BP_CrateW_BaseNitro_C|GetCube _array_element_3) 0 "/Game/Materials/M_Nitro_Transparent.M_Nitro_Transparent")
        (Collision|SetActorEnableCollision _array_element_3 false)))))

(event Custom|SpawnCrates
  ;[1 1 1] SpawnCrates
  (Utilities|FlowControl|Sequence
    (:then_0
      (for _array_element (Variables|Default|GetArrayCrate)
        (Rendering|Material|SetMaterial (Variables|/Game/Crates/NewCrate/BP_CrateW_Base.BP_CrateW_Base_C|GetCube _array_element) 0 "/Game/StarterContent/Materials/M_Wood_Floor_Walnut_Polished.M_Wood_Floor_Walnut_Polished")
        (Collision|SetActorEnableCollision _array_element true)))
    (:then_1
      (for _array_element_2 (Variables|Default|GetArrayTNT)
        (Rendering|Material|SetMaterial (Variables|/Game/Crates/NewCrate/BaseVariant/BP_CrateW_BaseTNT.BP_CrateW_BaseTNT_C|GetCube _array_element_2) 0 "/Engine/VREditor/BasicMeshes/M_TNT.M_TNT")
        (Collision|SetActorEnableCollision _array_element_2 true)))
    (:then_2
      (Rendering|Material|SetMaterial (Variables|/Game/Crates/NewCrate/BaseVariant/BP_CrateW_BaseNitro.BP_CrateW_BaseNitro_C|GetCube (stale _array_element)) 0 "/Game/Materials/M_Nitro.M_Nitro")
      (Collision|SetActorEnableCollision (stale _array_element) true))))

(event EventBeginPlay
  (CallFunction|DespawnCrates))

(event Collision|EventActorBeginOverlap
  (params (OtherActor :type Actor%20Object%20Reference)))

(event EventTick
  (params (DeltaSeconds :type Float%20%28single-precision%29)))

(event Game|Damage|EventAnyDamage
  (params (Damage :type Float%20%28single-precision%29) (DamageType :type Damage%20Type%20Object%20Reference) (InstigatedBy :type Controller%20Object%20Reference) (DamageCauser :type Actor%20Object%20Reference))
  (if (== DamageCauser (Game|GetPlayerCharacter 0))
    (Utilities|FlowControl|DoOnce false
      (:Completed
        (Variables|Default|SetCrateActivated true)
        (Variables|Default|SetTimer 2.0)
        (CallFunction|SpawnCrates)))))

(fn ConstructionScript)