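; BP_CrateBouncy is a crate that bounces the third-person character upward and breaks after a limited number of hits.
; On a hit from BP_ThirdPersonCharacter, it launches the character vertically, overriding Z velocity, and decrements its Hits counter.
; At zero, it spawns an actor at its own transform and destroys itself.
; The hit-normal check (Z >= -1) effectively accepts contact from any direction.
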(event `self.ReceiveHit`
  (params (MyComp :type "PrimitiveComponent Object Reference") (Other :type "Actor Object Reference") (OtherComp :type "PrimitiveComponent Object Reference") (bSelfMoved :type Boolean) (HitLocation :type "Vector Structure") (HitNormal :type "Vector Structure") (NormalImpulse :type "Vector Structure") (Hit :type "HitResult Structure (by ref)"))
  (if (>= (.z HitNormal) -1.0)
    (bind _asbp_third_person_character (cast `/Game/ThirdPerson/Blueprints/BP_ThirdPersonCharacter` Other))
    (`Character.LaunchCharacter` _asbp_third_person_character (0.0 0.0 600.0) false true)
    (bind _result (`/Engine/EditorBlueprintResources/StandardMacros.DecrementInt` (`self.Hits`))
      (:`  `
        (if (<= _result 0)
          (`|SpawnActorFromClass` "/Game/Blueprints/BP_Wumpa.BP_Wumpa_C" (`self.GetTransform` self) "Undefined" "MultiplyWithRoot" null null)
          (`self.K2_DestroyActor`))))))

(fn `UserConstructionScript`
  (`parent.UserConstructionScript`))