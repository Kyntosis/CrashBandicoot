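; BP_LevelCamera is a rail camera that follows the player character along a spline and becomes the player's view target on BeginPlay.
; Each tick it moves the SpringArm to the spline point closest to the character.
; The arm's yaw follows the spline direction at that point, with a fixed downward pitch and no roll.
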(event `self.ReceiveBeginPlay`
  (`PlayerController.SetViewTargetWithBlend` (`GameplayStatics.GetPlayerController` 0) self 0.0 "VTBlend_Linear" 0.0 false))

(event `self.ReceiveTick`
  (params (DeltaSeconds :type "Float (single-precision)"))
  (bind _spline (`self.Spline`))
  (bind _springarm (`self.SpringArm`))
  (bind _returnvalue (`self.K2_GetActorLocation` (`GameplayStatics.GetPlayerCharacter` 0)))
  (bind (_returnvalue_roll _returnvalue_pitch _returnvalue_yaw) (`KismetMathLibrary.BreakRotator` (`KismetMathLibrary.Conv_VectorToRotator` (`SplineComponent.FindDirectionClosestToWorldLocation` _spline _returnvalue "World"))))
  (`SceneComponent.K2_SetWorldLocation` _springarm (`SplineComponent.FindLocationClosestToWorldLocation` _spline _returnvalue "World") false false)
  (`SceneComponent.K2_SetWorldRotation` _springarm (`KismetMathLibrary.MakeRotator` 0.0 -40.0 _returnvalue_yaw) false false))

(fn `UserConstructionScript`)