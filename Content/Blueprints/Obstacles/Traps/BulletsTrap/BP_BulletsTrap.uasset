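; Bullet trap obstacle that fires continuously from two spawn points for as long as it is in play.
; BeginPlay runs an endless Delay loop timed by FireRateBullets, spawning an actor at each ProjectileSpawnPoint component on every cycle.
; Spawns take the point's location and rotation, use BulletScale as uniform scale, and always spawn, adjusting position for collisions if possible.
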(event `self.ReceiveBeginPlay`
  (bind _projectile_spawn_point (`self.Projectile Spawn Point`))
  (bind _projectile_spawn_point1 (`self.Projectile Spawn Point1`))
  (`KismetSystemLibrary.Delay` (`self.Fire Rate Bullets`) :!label _label)
  (`|SpawnActorFromClass` "/Game/Blueprints/Obstacles/Traps/BulletsTrap/BP_Bullets.BP_Bullets_C" (`KismetMathLibrary.MakeTransform` (`SceneComponent.K2_GetComponentLocation` _projectile_spawn_point) (`SceneComponent.K2_GetComponentRotation` _projectile_spawn_point) (`KismetMathLibrary.Conv_DoubleToVector` (`self.Bullet Scale`))) "AdjustIfPossibleButAlwaysSpawn" "MultiplyWithRoot" null null)
  (`|SpawnActorFromClass` "/Game/Blueprints/Obstacles/Traps/BulletsTrap/BP_Bullets.BP_Bullets_C" (`KismetMathLibrary.MakeTransform` (`SceneComponent.K2_GetComponentLocation` _projectile_spawn_point1) (`SceneComponent.K2_GetComponentRotation` _projectile_spawn_point1) (`KismetMathLibrary.Conv_DoubleToVector` (`self.Bullet Scale`))) "AdjustIfPossibleButAlwaysSpawn" "MultiplyWithRoot" null null)
  (goto _label))

(fn `UserConstructionScript`)