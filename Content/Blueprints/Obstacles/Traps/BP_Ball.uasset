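; BP_Ball is a trap that travels along the BP_LevelCamera spline and damages actors that touch its DeathTrigger.
; It spawns at the spline's end, raised by a height offset.
; When the player enters StartTrigger, a reversed Timeline with adjustable play rate lerps distance along the spline to set location and rotation, stopping when finished.
; Hitting the player also resets the Timeline's time to zero.
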(event `self.ReceiveBeginPlay`
  (bind _returnvalue (`GameplayStatics.GetActorOfClass` "/Game/Camera/BP_LevelCamera.BP_LevelCamera_C"))
  (bind _spline (`/Game/Camera/BP_LevelCamera.Spline` _returnvalue))
  (bind _returnvalue_2 (`SplineComponent.GetTransformAtDistanceAlongSpline` _spline (`SplineComponent.GetSplineLength` _spline) "World" false))
  (`self.K2_SetActorLocationAndRotation` (`KismetMathLibrary.MakeVector` (.x (.location _returnvalue_2)) (.y (.location _returnvalue_2)) (+ (.z (.location _returnvalue_2)) (`self.Offset`))) (.rotation _returnvalue_2)))

(event `StartMoving`
  (if (not (`self.MovedStart`))
    (bind _returnvalue (`GameplayStatics.GetActorOfClass` "/Game/Camera/BP_LevelCamera.BP_LevelCamera_C"))
    (`TimelineComponent.SetPlayRate` (`self.Timeline`) (`self.Play Rate`))
    (bind (_direction _alpha) (`Timeline|Timeline` :!via `Reverse` :!label _label)
      (:`Update`
        (bind _spline (`/Game/Camera/BP_LevelCamera.Spline` _returnvalue))
        (bind _returnvalue_2 (`SplineComponent.GetTransformAtDistanceAlongSpline` _spline (`KismetMathLibrary.Lerp` 0.0 (`SplineComponent.GetSplineLength` _spline) _alpha) "World" false))
        (`self.K2_SetActorLocationAndRotation` (`KismetMathLibrary.MakeVector` (.x (.location _returnvalue_2)) (.y (.location _returnvalue_2)) (+ (.z (.location _returnvalue_2)) (`self.Offset`))) (.rotation _returnvalue_2)))
      (:`Finished`
        (`self.StopMoving`)))))

(event `StopMoving`
  (set `self.MovedStart` false)
  (goto _label :!via `Stop`))

(event `self.DeathTrigger.OnComponentBeginOverlap`
  (params (OverlappedComponent :type "PrimitiveComponent Object Reference") (OtherActor :type "Actor Object Reference") (OtherComp :type "PrimitiveComponent Object Reference") (OtherBodyIndex :type Integer) (bFromSweep :type Boolean) (SweepResult :type "HitResult Structure (by ref)"))
  (`GameplayStatics.ApplyDamage` OtherActor 1.0)
  (if (== OtherActor (`GameplayStatics.GetPlayerCharacter` 0))
    (`TimelineComponent.SetNewTime` (`self.Timeline`) 0.0)))

(event `self.StartTrigger.OnComponentBeginOverlap`
  (params (OverlappedComponent :type "PrimitiveComponent Object Reference") (OtherActor :type "Actor Object Reference") (OtherComp :type "PrimitiveComponent Object Reference") (OtherBodyIndex :type Integer) (bFromSweep :type Boolean) (SweepResult :type "HitResult Structure (by ref)"))
  (if (== OtherActor (`GameplayStatics.GetPlayerCharacter` 0))
    (`self.StartMoving`)))

(fn `UserConstructionScript`)