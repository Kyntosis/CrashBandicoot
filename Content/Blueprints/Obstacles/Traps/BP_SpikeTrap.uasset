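; BP_SpikeTrap is a spike trap that rises when the player enters its trigger and retracts when the player leaves.
; TriggerTrap overlaps toggle the IsTrapOFF flag and play or reverse a timeline that sets the Trap component's relative Z location.
; A separate DeathTrigger applies damage to any overlapping BP_ThirdPersonCharacter, without checking whether the trap is raised.
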(event `OnActorBeginOverlap_Event` :!signature `self.OnActorBeginOverlap`
  (params (OverlappedActor :type "Actor Object Reference") (OtherActor :type "Actor Object Reference")))

(event `self.TriggerTrap.OnComponentBeginOverlap`
  (params (OverlappedComponent :type "PrimitiveComponent Object Reference") (OtherActor :type "Actor Object Reference") (OtherComp :type "PrimitiveComponent Object Reference") (OtherBodyIndex :type Integer) (bFromSweep :type Boolean) (SweepResult :type "HitResult Structure (by ref)"))
  (if (== OtherActor (`GameplayStatics.GetPlayerCharacter` 0))
    (if (`self.Is TrapOFF`)
      (`KismetSystemLibrary.PrintString` "Character in")
      (set `self.Is TrapOFF` false)
      (`KismetSystemLibrary.PrintString` "TrapON")
      (bind (_direction _activation_trap) (`Timeline|SpikeUP Animation Timeline` :!label _label)
        (:`Update`
          (`SceneComponent.K2_SetRelativeLocation` (`self.Trap`) (`KismetMathLibrary.MakeVector` 0.0 0.0 _activation_trap) false false))))))

(event `self.TriggerTrap.OnComponentEndOverlap`
  (params (OverlappedComponent :type "PrimitiveComponent Object Reference") (OtherActor :type "Actor Object Reference") (OtherComp :type "PrimitiveComponent Object Reference") (OtherBodyIndex :type Integer))
  (if (`self.Is TrapOFF`)
    _
    (elif (== OtherActor (`GameplayStatics.GetPlayerCharacter` 0))
      (`KismetSystemLibrary.PrintString` "Out")
      (set `self.Is TrapOFF` true)
      (`KismetSystemLibrary.PrintString` "TrapOFF")
      (goto _label :!via `Reverse`))))

(event `self.DeathTrigger.OnComponentBeginOverlap`
  (params (OverlappedComponent :type "PrimitiveComponent Object Reference") (OtherActor :type "Actor Object Reference") (OtherComp :type "PrimitiveComponent Object Reference") (OtherBodyIndex :type Integer) (bFromSweep :type Boolean) (SweepResult :type "HitResult Structure (by ref)"))
  (bind _asbp_third_person_character (cast `/Game/ThirdPerson/Blueprints/BP_ThirdPersonCharacter` OtherActor))
  (`GameplayStatics.ApplyDamage` _asbp_third_person_character 1.0))

(fn `UserConstructionScript`)