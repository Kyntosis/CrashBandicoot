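; Falling platform obstacle that drops after the player character steps into its trigger, and can optionally respawn.
; The first player overlap waits a drop delay, then adds and activates a projectile movement component and switches the mesh from WorldStatic to PhysicsBody collision.
; If respawnable, it spawns a new copy of itself at the saved start location after a further delay, without destroying the old one.
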(event `self.ReceiveBeginPlay`
  (set `self.StartingPosition` (`self.K2_GetActorLocation`))
  (`PrimitiveComponent.SetCollisionObjectType` (`self.FallingPlatform`) "ECC_WorldStatic"))

(event `self.Trigger.OnComponentBeginOverlap`
  (params (OverlappedComponent :type "PrimitiveComponent Object Reference") (OtherActor :type "Actor Object Reference") (OtherComp :type "PrimitiveComponent Object Reference") (OtherBodyIndex :type Integer) (bFromSweep :type Boolean) (SweepResult :type "HitResult Structure (by ref)"))
  (if (== OtherActor (`GameplayStatics.GetPlayerCharacter` 0))
    (`/Engine/EditorBlueprintResources/StandardMacros.DoOnce` false
      (:`Completed`
        (`KismetSystemLibrary.Delay` (`self.DropDelay`))
        (bind _returnvalue (`AddComponent|NODE_AddProjectileMovementComponent-0` :`self` self))
        (`ActorComponent.SetActive` _returnvalue true false)
        (`PrimitiveComponent.SetCollisionObjectType` (`self.FallingPlatform`) "ECC_PhysicsBody")
        (if (`self.Respawnable`)
          (`KismetSystemLibrary.Delay` (`self.RespawnDelay`))
          (`|SpawnActorFromClass` "BP_FallingPlatform_Respawn_C" (`KismetMathLibrary.Conv_VectorToTransform` (`self.StartingPosition`)) "Undefined" "MultiplyWithRoot" null 4.0 null))))))

(fn `UserConstructionScript`)