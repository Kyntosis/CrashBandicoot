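; BP_Elevator is an elevator actor that moves its Cube when anything begins overlapping its Box trigger.
; The IsDown flag selects one of two timelines, whose tracks directly set the Cube's relative location without sweeping.
; Each timeline update rewrites IsDown for the next overlap and prints it for debugging.
; Both timelines use Play rather than Play from Start, so neither rewinds between trips.
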(event `self.Box.OnComponentBeginOverlap`
  (params (OverlappedComponent :type "PrimitiveComponent Object Reference") (OtherActor :type "Actor Object Reference") (OtherComp :type "PrimitiveComponent Object Reference") (OtherBodyIndex :type Integer) (bFromSweep :type Boolean) (SweepResult :type "HitResult Structure (by ref)"))
  (if (`self.IsDown`)
    (bind (_direction _newtrack_0) (`Timeline|Timeline`)
      (:`Update`
        (`SceneComponent.K2_SetRelativeLocation` (`self.Cube`) _newtrack_0 false false)
        (bind _output_get (set `self.IsDown` false))
        (`KismetSystemLibrary.PrintString` (`KismetStringLibrary.Conv_BoolToString` _output_get))))
    (else
      (bind (_direction_2 _tack1) (`Timeline|Timeline_0`)
        (:`Update`
          (`SceneComponent.K2_SetRelativeLocation` (`self.Cube`) _tack1 false false)
          (bind _output_get_2 (set `self.IsDown` true))
          (`KismetSystemLibrary.PrintString` (`KismetStringLibrary.Conv_BoolToString` _output_get_2)))))))

(fn `UserConstructionScript`)