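; BP_TunnelVolume is a trigger volume that applies a camera modifier while the player character is inside it.
; On begin overlap with player 0's character, it adds BP_Tunnel_Cam_Modifier to that player's camera manager and stores the returned instance.
; On end overlap, it removes that stored modifier, so the tunnel camera effect lasts only while the player overlaps the volume.
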(event `self.ReceiveActorBeginOverlap`
  (params (OtherActor :type "Actor Object Reference"))
  (if (== OtherActor (`GameplayStatics.GetPlayerCharacter` 0))
    (bind _returnvalue (`PlayerCameraManager.AddNewCameraModifier` (`GameplayStatics.GetPlayerCameraManager` 0) "/Game/BP_Tunnel_Cam_Modifier.BP_Tunnel_Cam_Modifier_C"))
    (set `self.CamMod` _returnvalue)))

(event `self.ReceiveActorEndOverlap`
  (params (OtherActor :type "Actor Object Reference"))
  (if (== OtherActor (`GameplayStatics.GetPlayerCharacter` 0))
    (`PlayerCameraManager.RemoveCameraModifier` (`GameplayStatics.GetPlayerCameraManager` 0) (`self.CamMod`))))

(fn `UserConstructionScript`)