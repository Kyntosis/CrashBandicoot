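; BP_Enemy is a path-following enemy that the player can kill by bouncing on it and that damages the player on contact with its DeathZone.
; If a Path is valid, a Timeline moves and rotates it along that spline.
; Hits on the Enemy component passing a normal-impulse Z check launch the player upward and damage the enemy.
; Any damage spawns BP_Wumpa_Scaled in its place and destroys it.
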(event `self.ReceiveBeginPlay`
  (if (`KismetSystemLibrary.IsValid` (`self.Path`))
    (`self.Start Moving`)))

(event `self.ReceiveAnyDamage`
  (params (Damage :type "Float (single-precision)") (DamageType :type "DamageType Object Reference") (InstigatedBy :type "Controller Object Reference") (DamageCauser :type "Actor Object Reference"))
  (`|SpawnActorFromClass` "/Game/Blueprints/BP_Wumpa_Scaled.BP_Wumpa_Scaled_C" (`self.GetTransform`) "Undefined" "MultiplyWithRoot" null null)
  (`self.K2_DestroyActor`))

(event `Start Moving`
  (bind (_direction _alpha) (`Timeline|Timeline`)
    (:`Update`
      (bind (_returnvalue_location _returnvalue_rotation) (`KismetMathLibrary.BreakTransform` (`SplineComponent.GetTransformAtDistanceAlongSpline` (`/Game/Enemy/BP_EnemyPath.Spline` (`self.Path`)) (`KismetMathLibrary.Lerp` 0.0 (`SplineComponent.GetSplineLength` (`/Game/Enemy/BP_EnemyPath.Spline` (`self.Path`))) _alpha) "World" false)))
      (`self.K2_SetActorLocationAndRotation` _returnvalue_location _returnvalue_rotation))))

(event `self.Enemy.OnComponentHit`
  (params (HitComponent :type "PrimitiveComponent Object Reference") (OtherActor :type "Actor Object Reference") (OtherComp :type "PrimitiveComponent Object Reference") (NormalImpulse :type "Vector Structure") (Hit :type "HitResult Structure (by ref)"))
  (bind _z (.z NormalImpulse))
  (`KismetSystemLibrary.PrintString` (`KismetStringLibrary.Conv_DoubleToString` _z))
  (if (>= _z -1.0)
    (bind _asbp_third_person_character (cast `/Game/ThirdPerson/Blueprints/BP_ThirdPersonCharacter` OtherActor))
    (`Character.LaunchCharacter` _asbp_third_person_character (0.0 0.0 600.0) false true)
    (`GameplayStatics.ApplyDamage` self 1.0 null _asbp_third_person_character)))

(event `self.DeathZone.OnComponentBeginOverlap`
  (params (OverlappedComponent :type "PrimitiveComponent Object Reference") (OtherActor :type "Actor Object Reference") (OtherComp :type "PrimitiveComponent Object Reference") (OtherBodyIndex :type Integer) (bFromSweep :type Boolean) (SweepResult :type "HitResult Structure (by ref)"))
  (bind _asbp_third_person_character (cast `/Game/ThirdPerson/Blueprints/BP_ThirdPersonCharacter` OtherActor))
  (`GameplayStatics.ApplyDamage` _asbp_third_person_character 1.0))

(fn `UserConstructionScript`)