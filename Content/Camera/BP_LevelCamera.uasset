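; Level camera actor that becomes the player's view target on BeginPlay and follows the player character along a spline.
; Each tick the spring arm snaps to the spline point nearest the character, yawed along the spline direction with a fixed downward pitch.
; Ball mode adds a height offset, steeper pitch and its own arm length.
; Otherwise, the arm only updates when Is2D is off, so 2D mode leaves it untouched.
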(event `self.ReceiveBeginPlay`
  (`PlayerController.SetViewTargetWithBlend` (`GameplayStatics.GetPlayerController` 0) self 0.0 "VTBlend_Linear" 0.0 false))

(event `self.ReceiveTick`
  (params (DeltaSeconds :type "Float (single-precision)"))
  (bind _spline (`self.Spline`))
  (bind _springarm (`self.SpringArm`))
  (bind _returnvalue (`self.K2_GetActorLocation` (`GameplayStatics.GetPlayerCharacter` 0)))
  (bind (_returnvalue_x _returnvalue_y _returnvalue_z) (`KismetMathLibrary.BreakVector` (`SplineComponent.FindLocationClosestToWorldLocation` _spline _returnvalue "World")))
  (bind (_returnvalue_roll _returnvalue_pitch _returnvalue_yaw) (`KismetMathLibrary.BreakRotator` (`KismetMathLibrary.Conv_VectorToRotator` (`SplineComponent.FindDirectionClosestToWorldLocation` _spline _returnvalue "World"))))
  (if (`self.Ball`)
    (`SceneComponent.K2_SetWorldLocation` _springarm (`KismetMathLibrary.MakeVector` _returnvalue_x _returnvalue_y (+ _returnvalue_z (`self.BallZOffset`))) false false)
    (`SceneComponent.K2_SetWorldRotation` _springarm (`KismetMathLibrary.MakeRotator` 0.0 -30.0 _returnvalue_yaw) false false)
    (set `SpringArmComponent.TargetArmLength` (`self.Ball Arm Length`) (`self.SpringArm`))
    (elif (not (`self.Is2D`))
      (`SceneComponent.K2_SetWorldLocation` _springarm (`KismetMathLibrary.MakeVector` _returnvalue_x _returnvalue_y _returnvalue_z) false false)
      (`SceneComponent.K2_SetWorldRotation` _springarm (`KismetMathLibrary.MakeRotator` 0.0 -20.0 _returnvalue_yaw) false false))))

(fn `UserConstructionScript`)